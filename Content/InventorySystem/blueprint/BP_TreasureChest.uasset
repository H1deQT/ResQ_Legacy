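; BP_TreasureChest is an interactable chest that the player opens and closes with F while inside its trigger.
; Overlap with the Miguel character sets the in-range flag, and out-of-range presses print a warning.
; A FlipFlop alternates playing and reversing a timeline that rotates the cover, ignoring input during animation.
; The key requirement is not functional: its branch is fixed to false, so no key is needed.
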(event OnComponentBeginOverlap(Trigger)
  (params (OverlappedComponent :type Primitive%20Component%20Object%20Reference) (OtherActor :type Actor%20Object%20Reference) (OtherComp :type Primitive%20Component%20Object%20Reference) (OtherBodyIndex :type Integer) (bFromSweep :type Boolean) (SweepResult :type Hit%20Result%20Structure%20%28by%20ref%29))
  (Utilities|Casting|CastToMiguel OtherActor)
  (Development|PrintString "Player is in range")
  (Variables|Default|SetB_PlayerInRange true)
  (Variables|Default|SetB_PlayerHasAKey false))

(event OnComponentEndOverlap(Trigger)
  (params (OverlappedComponent :type Primitive%20Component%20Object%20Reference) (OtherActor :type Actor%20Object%20Reference) (OtherComp :type Primitive%20Component%20Object%20Reference) (OtherBodyIndex :type Integer))
  (Utilities|Casting|CastToMiguel OtherActor)
  (Development|PrintString "Player is out of range")
  (Variables|Default|SetB_PlayerInRange false)
  (Variables|Default|SetB_PlayerHasAKey false))

(event Custom|ToggleChest
  (params (Reverse? :type Boolean))
  (bind _openandclosetimeline (Variables|Default|GetOpenAndCloseTimeline))
  (if Reverse?
    (Components|Timeline|SetPlayRate _openandclosetimeline 1.0)
    (Variables|Default|SetB_IsAnimating true)
    (bind _closeandopen (Timeline|OpenAndCloseTimeline ReverseFromEnd)
      (:Update
        (Transformation|SetRelativeRotation (Variables|Default|GetChest_Cover) (Math|Rotator|MakeRotator _closeandopen 0.0 0.0) false false))
      (:Finished
        (Variables|Default|SetB_IsAnimating false)))
    (else
      (Components|Timeline|SetPlayRate _openandclosetimeline 1.0)
      (Variables|Default|SetB_IsAnimating true)
      (Timeline|OpenAndCloseTimeline PlayFromStart))))

(event EventBeginPlay
  (Input|EnableInput (Game|GetPlayerController 0)))

(event EventTick
  (params (DeltaSeconds :type Float%20%28single-precision%29)))

(event Input|KeyboardEvents|F
  (params (Key :type Key%20Structure :default "None"))
  (:Pressed
    (if (Variables|Default|GetB_PlayerInRange)
      (if false
        (Development|PrintString "Get the key first" true true "(R=1.000000,G=0.000000,B=0.216807,A=1.000000)")
        (elif (not (Variables|Default|GetB_IsAnimating))
          (Utilities|FlowControl|FlipFlop
            (:A
              (CallFunction|ToggleChest false)
              (Variables|Default|SetB_IsChestOpened true)
              (Variables|Default|Setstatus "close"))
            (:B
              (CallFunction|ToggleChest true)
              (Variables|Default|SetB_IsChestOpened false)
              (Variables|Default|Setstatus "open")))))
      (else
        (Development|PrintString (Utilities|String|ToString(Text) (Utilities|Text|FormatText "You can't {status} chest while you're out of range." (Variables|Default|Getstatus))) true true "(R=1.000000,G=0.058196,B=0.002460,A=1.000000)")))))

(fn ConstructionScript)