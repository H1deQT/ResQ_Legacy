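; BP_Key is a pickup key that shows an outline material when the player character enters its Trigger volume.
; Entering adds a duplicate mesh component and outlines the original; leaving restores the material but keeps the duplicate.
; A separate KeyCollision volume, unfiltered by actor type, gates the E key.
; Pressing E inside it destroys the key and sets BHasKey on BP_ThirdPersonCharacter, otherwise it prints a warning.
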(event OnComponentBeginOverlap(Trigger)
  (params (OverlappedComponent :type Primitive%20Component%20Object%20Reference) (OtherActor :type Actor%20Object%20Reference) (OtherComp :type Primitive%20Component%20Object%20Reference) (OtherBodyIndex :type Integer) (bFromSweep :type Boolean) (SweepResult :type Hit%20Result%20Structure%20%28by%20ref%29))
  (bind _staticmesh (Variables|Default|GetStaticMesh))
  (Utilities|Casting|CastToBP_ThirdPersonCharacter OtherActor)
  (bind _returnvalue (AddComponent|AddStaticMeshComponent false (Transformation|GetRelativeTransform _staticmesh)))
  (bind _output_get (Variables|Default|SetAddStaticMesh _returnvalue))
  (Components|StaticMesh|SetStaticMesh _output_get (Variables|/Script/Engine.StaticMeshComponent|GetStaticMesh _staticmesh))
  (Rendering|Material|SetMaterial _staticmesh 0 "/Game/InventorySystem/material/M_KeyOutline_Inst.M_KeyOutline_Inst")
  (Variables|Default|SetB_PlayerInRange true))

(event OnComponentEndOverlap(Trigger)
  (params (OverlappedComponent :type Primitive%20Component%20Object%20Reference) (OtherActor :type Actor%20Object%20Reference) (OtherComp :type Primitive%20Component%20Object%20Reference) (OtherBodyIndex :type Integer))
  (bind _staticmesh (Variables|Default|GetStaticMesh))
  (Utilities|Casting|CastToBP_ThirdPersonCharacter OtherActor)
  (Components|StaticMesh|SetStaticMesh _staticmesh (Variables|/Script/Engine.StaticMeshComponent|GetStaticMesh _staticmesh))
  (Rendering|Material|SetMaterial (Variables|Default|GetStaticMesh) 0 "/Game/InventorySystem/Object/key/KEY_Mat.KEY_Mat")
  (Variables|Default|SetB_PlayerInRange false))

(event OnComponentBeginOverlap(KeyCollision)
  (params (OverlappedComponent :type Primitive%20Component%20Object%20Reference) (OtherActor :type Actor%20Object%20Reference) (OtherComp :type Primitive%20Component%20Object%20Reference) (OtherBodyIndex :type Integer) (bFromSweep :type Boolean) (SweepResult :type Hit%20Result%20Structure%20%28by%20ref%29))
  (Variables|Default|SetB_isPlayerInsideOfKeyCollision true))

(event OnComponentEndOverlap(KeyCollision)
  (params (OverlappedComponent :type Primitive%20Component%20Object%20Reference) (OtherActor :type Actor%20Object%20Reference) (OtherComp :type Primitive%20Component%20Object%20Reference) (OtherBodyIndex :type Integer))
  (Variables|Default|SetB_isPlayerInsideOfKeyCollision false))

(event EventBeginPlay
  (Input|EnableInput (Game|GetPlayerController 0)))

(event Collision|EventActorBeginOverlap
  (params (OtherActor :type Actor%20Object%20Reference)))

(event EventTick
  (params (DeltaSeconds :type Float%20%28single-precision%29)))

(event Input|KeyboardEvents|E
  (params (Key :type Key%20Structure :default "None"))
  (:Pressed
    (if (Variables|Default|GetB_isPlayerInsideOfKeyCollision)
      (Actor|DestroyActor)
      (bind _returnvalue (Actor|GetActorOfClass "/Game/ThirdPerson/Blueprints/BP_ThirdPersonCharacter.BP_ThirdPersonCharacter_C"))
      (Variables|/Game/ThirdPerson/Blueprints/BP_ThirdPersonCharacter.BP_ThirdPersonCharacter_C|SetB_HasKey _returnvalue true)
      (else
        (Development|PrintString "You can't pickup the key while you're out of key collision" true true "(R=1.000000,G=0.066259,B=0.000000,A=1.000000)")))))

(fn ConstructionScript)